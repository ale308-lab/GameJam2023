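; An interactable lever actor that toggles between on and off states.
; Interact calls ChangeState, which inverts OnOffState and runs FlipOn or FlipOff, then always returns false.
; Each flip function sets the state explicitly and plays its non-looping animation on the Lever component.
; The file contains no logic that drives other actors from the lever's state.
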(fn `changeState`
  (bind _output_get (set `self.OnOffState` (not (`self.OnOffState`))))
  (if _output_get
    (`self.flipOn`)
    (else
      (`self.flipOff`))))

(fn `flipOff`
  (set `self.OnOffState` false)
  (`SkeletalMeshComponent.PlayAnimation` (`self.Lever`) "/Game/Assets/Animations/LeverOff.LeverOff" false))

(fn `flipOn`
  (set `self.OnOffState` true)
  (`SkeletalMeshComponent.PlayAnimation` (`self.Lever`) "/Game/Assets/Animations/LeverOn.LeverOn" false))

(fn `Interact`
  (returns (Success :type Boolean))
  (`self.changeState`)
  (return false))

(fn `UserConstructionScript`)