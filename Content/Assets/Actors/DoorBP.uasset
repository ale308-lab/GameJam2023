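; Door actor Blueprint that opens and closes an animated door.
; Open and Close each set the OpenCloseState flag, play a one-shot open or close animation on the Door mesh, and disable or restore collision on the Colission component.
; ToggleDoor flips the flag and calls Open or Close to match.
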(fn `Close`
  (set `self.OpenCloseState` false)
  (`SkeletalMeshComponent.PlayAnimation` (`self.Door`) "/Game/Assets/Animations/DoorClose.DoorClose" false)
  (`PrimitiveComponent.SetCollisionEnabled` (`self.Colission`) "QueryAndPhysics"))

(fn `Open`
  (set `self.OpenCloseState` true)
  (`SkeletalMeshComponent.PlayAnimation` (`self.Door`) "/Game/Assets/Animations/DoorOpen.DoorOpen" false)
  (`PrimitiveComponent.SetCollisionEnabled` (`self.Colission`) "NoCollision"))

(fn `ToggleDoor`
  (bind _output_get (set `self.OpenCloseState` (not (`self.OpenCloseState`))))
  (if _output_get
    (`self.Open`)
    (else
      (`self.Close`))))

(fn `UserConstructionScript`)